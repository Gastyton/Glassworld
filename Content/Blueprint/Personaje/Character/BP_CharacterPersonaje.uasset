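; Player character Blueprint for side-scrolling movement along the world X axis, with jumping.
; On BeginPlay it registers an Enhanced Input mapping context with the local player.
; The move action feeds AddMovementInput on X, and the sign of the current X acceleration snaps control rotation yaw to 0 or 180 to face left or right.
; The jump action calls Jump when it starts.
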(event Input|EnhancedActionEvents|EnhancedInputActionIA_Movimiento
  (params (ActionValue :type Float%20%28double-precision%29) (ElapsedSeconds :type Float%20%28double-precision%29) (TriggeredSeconds :type Float%20%28double-precision%29) (InputAction :type Input%20Action%20Object%20Reference :default "/Game/Blueprint/Inputs/InputAction/IA_Movimiento.IA_Movimiento"))
  (bind _returnvalue (Pawn|GetController))
  ;[1 1 1] Movmiento Derecha Izquierda pj
  (Pawn|Input|AddMovementInput "1.000000,0.000000,0.000000" ActionValue false)
  (Math|Float|CompareFloat (.x (Pawn|Components|CharacterMovement|GetCurrentAcceleration (Variables|Character|GetCharacterMovement))) 0.0
    (:>
      (Pawn|SetControlRotation _returnvalue (Math|Rotator|MakeRotator 0.0 0.0 0.0)))
    (:<
      (Pawn|SetControlRotation _returnvalue (Math|Rotator|MakeRotator 0.0 0.0 1.8e+02)))))

(event Input|EnhancedActionEvents|EnhancedInputActionIA_Saltar
  (params (ActionValue :type Float%20%28double-precision%29) (ElapsedSeconds :type Float%20%28double-precision%29) (TriggeredSeconds :type Float%20%28double-precision%29) (InputAction :type Input%20Action%20Object%20Reference :default "/Game/Blueprint/Inputs/InputAction/IA_Saltar.IA_Saltar"))
  (:Started
    (Character|Jump)))

(event EventBeginPlay
  (bind _asplayer_controller (Utilities|Casting|CastToPlayerController (Pawn|GetController)))
  (Input|AddMappingContext (PlayerController|LocalPlayerSubsystems|GetEnhancedInputLocalPlayerSubsystem _asplayer_controller) "/Game/Blueprint/Inputs/Mappingcontext/IMC_PersonajeMappingContext.IMC_PersonajeMappingContext" 0 "(bIgnoreAllPressedKeysUntilRelease=True,bForceImmediately=False,bNotifyUserSettings=False)"))

(fn ConstructionScript)